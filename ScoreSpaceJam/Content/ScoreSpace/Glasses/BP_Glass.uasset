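; BP_Glass is a drink glass that BP_IceCubeCharacter floats in, configured by its GlassType.
; The construction script applies the content material and sets 3D labels for content name and points.
; Overlap start passes GlassType and HasFloated (as CountPoints) to the character, then sets that flag and hides the points label; overlap end stops floating.
; When ShouldMove is set, Tick moves the glass vertically at MovingSpeed with sweep.
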(event OnComponentBeginOverlap(OverlappingCollider)
  (params (OverlappedComponent :type Primitive%20Component%20Object%20Reference) (OtherActor :type Actor%20Object%20Reference) (OtherComp :type Primitive%20Component%20Object%20Reference) (OtherBodyIndex :type Integer) (bFromSweep :type Boolean) (SweepResult :type Hit%20Result%20Structure%20%28by%20ref%29))
  (bind _asbp_ice_cube_character (Utilities|Casting|CastToBP_IceCubeCharacter OtherActor))
  (Default|OnStartFloating _asbp_ice_cube_character (Variables|Default|GetGlassType) (Variables|Default|GetHasFloated))
  (CallFunction|OnFloat))

(event OnComponentEndOverlap(OverlappingCollider)
  (params (OverlappedComponent :type Primitive%20Component%20Object%20Reference) (OtherActor :type Actor%20Object%20Reference) (OtherComp :type Primitive%20Component%20Object%20Reference) (OtherBodyIndex :type Integer))
  (bind _asbp_ice_cube_character (Utilities|Casting|CastToBP_IceCubeCharacter OtherActor))
  (Default|OnEndFloating _asbp_ice_cube_character (Variables|Default|GetGlassType)))

(event EventBeginPlay)

(event EventTick
  (params (DeltaSeconds :type Float%20%28single-precision%29))
  (if (Variables|Default|GetShouldMove)
    (if true
      (Transformation|AddWorldOffset (Variables|Default|GetDefaultSceneRoot) (Math|Vector|MakeVector 0.0 0.0 (* DeltaSeconds (Variables|Default|GetMovingSpeed))) true false))))

(fn ConstructionScript
  (bind _glasstype (Variables|Default|GetGlassType))
  (Utilities|FlowControl|Sequence
    (:then_0
      ;[1 1 1] Set Glass Material
      (Rendering|Material|SetMaterial (Variables|Default|GetContent) 0 (Variables|/Game/ScoreSpace/Glasses/DataAssets/GlassTypeDataAsset.GlassTypeDataAsset_C|GetContentMaterial (Variables|Default|GetGlassType))))
    (:then_1
      ;[1 1 1] Set Glass 3D Text
      (Utilities|FlowControl|Sequence
        (:then_0
          (Variables|/Script/Text3D.Text3DComponent|SetText (Variables|Default|GetContentNameText3D) (Utilities|Text|ToText(String) (Variables|/Game/ScoreSpace/Glasses/DataAssets/GlassTypeDataAsset.GlassTypeDataAsset_C|GetContentName _glasstype))))
        (:then_1
          (Variables|/Script/Text3D.Text3DComponent|SetText (Variables|Default|GetPointsText3D) (Utilities|Text|ToText(String) (Utilities|String|Append (Utilities|String|ToString(Integer) (Variables|/Game/ScoreSpace/Glasses/DataAssets/GlassTypeDataAsset.GlassTypeDataAsset_C|GetPointsOnFloat _glasstype)) " DP"))))))))

(fn OnFloat
  (Variables|Default|SetHasFloated true)
  (Rendering|SetVisibility (Variables|Default|GetPointsText3D) false false))