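; Spawner actor that keeps placing BP_Glass actors at random points inside a box, up to a count limit.
; Tick runs through a Delay, then retries random points that must be near the last glass and clear of all others.
; Glass type comes from sequential independent rolls over SpawnProbabilities, defaulting to water; the sum check is unwired.
; It also despawns glasses and can move the box above the latest floated one.
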(event EventBeginPlay)

(event Collision|EventActorBeginOverlap
  (params (OtherActor :type Actor%20Object%20Reference)))

(event EventTick
  (params (DeltaSeconds :type Float%20%28single-precision%29))
  (Utilities|FlowControl|Delay (Variables|SpawnParameters|GetSpawnRate))
  (CallFunction|CheckMaxSpawned)
  (if (Variables|SpawnParameters|GetShouldSpawn)
    (CallFunction|Spawn)))

(fn ConstructionScript)

(fn SpawnGlassatPoint
  (params (SpawnPoint :type Vector))
  (bind _returnvalue (Game|SpawnActorfromClass "/Game/ScoreSpace/Glasses/BP_Glass.BP_Glass_C" (Math|Transform|MakeTransform SpawnPoint "0, 0, 0" "1.000000,1.000000,1.000000") "Undefined" "MultiplyWithRoot" 0 (CallFunction|GetRandomGlassType) (Variables|SpawnParameters|GetGlassesMovingSpeed) 0))
  (Utilities|Array|Add (Variables|SpawnParameters|GetSpawnedGlasses) _returnvalue))

(fn GetRandomSpawnPoint
  (bind _spawningbox (Variables|Default|GetSpawningBox))
  (return (Math|Random|RandomPointinBoundingBox (Transformation|GetWorldLocation _spawningbox) (Variables|/Script/Engine.BoxComponent|GetBoxExtent _spawningbox))))

(fn Spawn
  (Utilities|FlowControl|ForLoopwithBreak 0 10 :!label _label
    (:LoopBody
      (bind _spawnpoint (CallFunction|GetRandomSpawnPoint))
      (if (CallFunction|IsSpawnPointValid _spawnpoint)
        (CallFunction|SpawnGlassatPoint _spawnpoint)
        (goto _label Break)))))

(fn IsSpawnPointValid
  (params (SpawnPoint :type Vector))
  (bind _spawnedglasses (Variables|SpawnParameters|GetSpawnedGlasses))
  (if (Utilities|Array|IsEmpty _spawnedglasses)
    (return true)
    (else
      (Utilities|FlowControl|Sequence
        (:then_0
          ;[1 1 1] Check Max Distance in regards to last
          (if (> (Math|Vector|Distance(Vector) SpawnPoint (Transformation|GetWorldLocation (Variables|/Game/ScoreSpace/Glasses/BP_Glass.BP_Glass_C|GetDefaultSceneRoot (Utilities|Array|Get(acopy) _spawnedglasses (Utilities|Array|LastIndex _spawnedglasses))))) (Variables|SpawnParameters|GetMaxSpawnDistance))
            (return false)))
        (:then_1
          ;[1 1 1] Check Min Distance in regards to all other spawned
          (for _array_element _spawnedglasses
            (if (< (Math|Vector|Distance(Vector) SpawnPoint (Transformation|GetWorldLocation (Variables|/Game/ScoreSpace/Glasses/BP_Glass.BP_Glass_C|GetDefaultSceneRoot _array_element))) (Variables|SpawnParameters|GetMinSpawnDistance))
              (return false))))
        (:then_2
          (return true))))))

(fn CheckMaxSpawned
  (Variables|SpawnParameters|SetShouldSpawn (<= (Utilities|Array|Length (Variables|SpawnParameters|GetSpawnedGlasses)) (Variables|SpawnParameters|GetMaxGlassesSpawned))))

(fn Despawn
  (params (Glass :type BP%20Glass%20Object%20Reference))
  (Utilities|Array|RemoveItem (Variables|SpawnParameters|GetSpawnedGlasses) Glass)
  (Actor|DestroyActor Glass))

(fn RelocatewithLastTouched
  (bind _arrayelement (Utilities|Array|ReverseforEachLoop (Variables|SpawnParameters|GetSpawnedGlasses))
    (:LoopBody
      (if (Variables|/Game/ScoreSpace/Glasses/BP_Glass.BP_Glass_C|GetHasFloated _arrayelement)
        (Transformation|SetWorldLocation (Variables|Default|GetSpawningBox) (+ (Transformation|GetWorldLocation (Variables|/Game/ScoreSpace/Glasses/BP_Glass.BP_Glass_C|GetDefaultSceneRoot _arrayelement)) (Math|Vector|MakeVector 0.0 0.0 (LocalVariables|GetZRelocationOffset))) false true)
        (return)))))

(fn GetRandomGlassType
  (Utilities|FlowControl|Sequence
    (:then_0
      ;[1 1 1] Check Spawn Probabilities
      (bind _keys (Utilities|Map|Keys (Variables|SpawnParameters|GetSpawnProbabilities)))
      (for _array_element _keys
        _))
    (:then_1
      ;[1 1 1] Get Random Glass Type
      (bind _keys_2 (Utilities|Map|Keys (Variables|SpawnParameters|GetSpawnProbabilities)))
      (for _array_element_2 _keys_2
        (if (<= (Math|Random|RandomFloat) (.Value (Utilities|Map|Find (Variables|SpawnParameters|GetSpawnProbabilities) _array_element_2)))
          (return _array_element_2)))
      (return "/Game/ScoreSpace/Glasses/DataAssets/DA_WaterGlass.DA_WaterGlass"))))