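; Game Instance for the Ice Cube game that handles its LootLocker online leaderboard and local player data.
; On Init it logs in as a guest, then requests the player's name, highscore and rank, plus the top leaderboard entries.
; SubmitScore sends the player name and most recent score, updating cached bests on improvement.
; Async callbacks log failures, and results are wrapped as BP_LeaderboardEntryData objects, also returned by GetPlayerData.
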(event Custom|Event%20GetScoreListCompleted
  (params (Response :type Loot%20Locker%20Get%20Score%20List%20Response%20Structure))
  (bind (_pagination _items _success _statuscode _fulltextfromserver) (Utilities|Struct|BreakLootLockerGetScoreListResponse Response))
  (bind _leaderboard (Variables|Leaderboard|GetLeaderboard))
  ;[1 1 1] LootLocker: Load Leaderboard and Personal Best
  (if _success
    (Utilities|Array|Clear _leaderboard)
    (for _array_element _items
      (bind _returnvalue (Game|ConstructObjectfromClass "/Game/ScoreSpace/UI/BP_LeaderboardEntryData.BP_LeaderboardEntryData_C" (.name (.player _array_element)) (.score _array_element) (.rank _array_element)))
      (Utilities|Array|Add _leaderboard _returnvalue))
    (else
      (Utilities|String|LogString _fulltextfromserver))))

(event Custom|Event%20SubmitScore
  (Utilities|FlowControl|Sequence
    (:then_0
      ;[1 1 1] LootLocker: Set Player Name
      (Class|LootLockerManager|SetPlayerName (Variables|Player|GetPlayerName) (delegate Custom|Event%20SetPlayerNameCompleted)))
    (:then_1
      ;[1 1 1] LootLocker: Submit Score to Leaderboard
      (Class|LootLockerManager|SubmitScore (Variables|Player|GetLootLocker_PlayerIdentifier) (Variables|Leaderboard|GetLootLocker_LeaderboardKey) (Variables|Player|GetMostRecentScore) "" (delegate Custom|Event%20SubmitScoreCompleted)))))

(event Custom|Event%20SetPlayerNameCompleted
  (params (Value :type Loot%20Locker%20Name%20Response%20Structure))
  (bind (_name _success _statuscode _fulltextfromserver) (Utilities|Struct|BreakLootLockerNameResponse Value))
  ;[1 1 1] LootLocker: Set Player Name
  (if (not _success)
    (Utilities|String|LogString _fulltextfromserver)))

(event Custom|Event%20GuestLogin
  ;[1 1 1] LootLocker: Guest Login
  (Class|LootLockerManager|GuestLogin (delegate Custom|Event%20GuestLoginCompleted)))

(event Custom|Event%20GuestLoginCompleted
  (params (Var :type Loot%20Locker%20Authentication%20Response%20Structure))
  (bind (_player_id _public_uid _player_ulid _seen_before _check_grant_notifications _check_deactivation_notifications _xp _level _level_thresholds _account_balance _player_identifier _session_token _success _statuscode _fulltextfromserver) (Utilities|Struct|BreakLootLockerAuthenticationResponse Var))
  ;[1 1 1] LootLocker: Guest Login
  (if _success
    (bind _output_get (Variables|Player|SetLootLocker_PlayerId _player_id))
    (bind _output_get_2 (Variables|Player|SetLootLocker_PlayerIdentifier _player_identifier))
    (Utilities|FlowControl|Sequence
      (:then_0
        (Utilities|String|LogString (Utilities|String|Append "Logged in as: " _output_get_2 ", ID: " (Utilities|String|ToString(Integer) _output_get))))
      (:then_1
        (CallFunction|EventUpdatePlayerData))
      (:then_2
        (CallFunction|EventLoadLeaderboard)))
    (else
      (Utilities|String|LogString _fulltextfromserver))))

(event Custom|Event%20SubmitScoreCompleted
  (params (Response :type Loot%20Locker%20Submit%20Score%20Response%20Structure))
  (bind (_member_id _rank _score _metadata _success _statuscode _fulltextfromserver) (Utilities|Struct|BreakLootLockerSubmitScoreResponse Response))
  ;[1 1 1] LootLocker: Submit Score to Leaderboard
  (if _success
    (Utilities|FlowControl|Sequence
      (:then_0
        (if (< _rank (Variables|Player|GetPlayerRank))
          (Variables|Player|SetPlayerRank _rank)))
      (:then_1
        (if (> _score (Variables|Player|GetHighscore))
          (Variables|Player|SetHighscore _score))))
    (else
      (Utilities|String|LogString _fulltextfromserver))))

(event Custom|Event%20LoadLeaderboard
  ;[1 1 1] LootLocker: Load Leaderboard and Personal Best
  (Class|LootLockerManager|GetScoreList (Variables|Leaderboard|GetLootLocker_LeaderboardKey) 25 0 (delegate Custom|Event%20GetScoreListCompleted)))

(event Custom|Event%20UpdatePlayerData
  ;[1 1 1] LootLocker: Get Member Rank
  (Class|LootLockerManager|GetMemberRank (Variables|Leaderboard|GetLootLocker_LeaderboardKey) (Utilities|String|ToString(Integer) (Variables|Player|GetLootLocker_PlayerId)) (delegate Custom|Event%20GetMemberRankCompleted)))

(event Custom|Event%20GetMemberRankCompleted
  (params (Response :type Loot%20Locker%20Get%20Member%20Rank%20Response%20Structure))
  (bind (_member_id _rank _score _player _metadata _success _statuscode _fulltextfromserver) (Utilities|Struct|BreakLootLockerGetMemberRankResponse Response))
  ;[1 1 1] LootLocker: Get Member Rank
  (if _success
    (Utilities|FlowControl|Sequence
      (:then_0
        (bind _output_get (Variables|Player|SetPlayerName (.name _player))))
      (:then_1
        (bind _output_get_2 (Variables|Player|SetHighscore _score)))
      (:then_2
        (bind _output_get_3 (Variables|Player|SetPlayerRank _rank)))
      (:then_3
        (Utilities|String|LogString (Utilities|String|Append "Player Data: " _output_get ", Highscore: " (Utilities|String|ToString(Integer) _output_get_2) ", Rank: " (Utilities|String|ToString(Integer) _output_get_3)))))
    (else
      (Utilities|String|LogString _fulltextfromserver))))

(event EventInit
  (CallFunction|EventGuestLogin))

(fn GetPlayerData
  (bind _returnvalue (Game|ConstructObjectfromClass "/Game/ScoreSpace/UI/BP_LeaderboardEntryData.BP_LeaderboardEntryData_C" (Variables|Player|GetPlayerName) (Variables|Player|GetHighscore) (Variables|Player|GetPlayerRank)))
  (return _returnvalue))