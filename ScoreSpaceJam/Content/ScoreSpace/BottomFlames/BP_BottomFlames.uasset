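; BP_BottomFlames is a flame hazard that burns the ice cube character and clears glasses that touch it.
; It plays a fire ambience on BeginPlay and reacts to overlaps on its FlameBlock component.
; An overlapping character triggers a burn sound and respawns above the middle entry of GlassesSpawner's spawned glasses, raised by a Z offset.
; An overlapping glass is despawned through GlassesSpawner.
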(event OnComponentBeginOverlap(FlameBlock)
  (params (OverlappedComponent :type Primitive%20Component%20Object%20Reference) (OtherActor :type Actor%20Object%20Reference) (OtherComp :type Primitive%20Component%20Object%20Reference) (OtherBodyIndex :type Integer) (bFromSweep :type Boolean) (SweepResult :type Hit%20Result%20Structure%20%28by%20ref%29))
  (bind _asbp_ice_cube_character (Utilities|Casting|CastToBP_IceCubeCharacter OtherActor)
    (:then
      (Audio|PlaySound2D "/Game/ScoreSpace/Sound/SFX_BurnUp.SFX_BurnUp" 1.0 1.0 0.0 0 0)
      (CallFunction|RespawnCharacter _asbp_ice_cube_character))
    (:CastFailed
      (bind _asbp_glass (Utilities|Casting|CastToBP_Glass OtherActor))
      (CallFunction|DespawnGlass _asbp_glass))))

(event OnComponentEndOverlap(FlameBlock)
  (params (OverlappedComponent :type Primitive%20Component%20Object%20Reference) (OtherActor :type Actor%20Object%20Reference) (OtherComp :type Primitive%20Component%20Object%20Reference) (OtherBodyIndex :type Integer))
  (Utilities|Casting|CastToBP_IceCubeCharacter OtherActor))

(event EventBeginPlay
  (Audio|PlaySound2D "/Game/ScoreSpace/Sound/Ambient_FireBurning.Ambient_FireBurning" 1.0 1.0 0.0 0 0 false))

(event EventTick
  (params (DeltaSeconds :type Float%20%28single-precision%29)))

(fn ConstructionScript)

(fn DespawnGlass
  (params (Glass :type BP%20Glass%20Object%20Reference))
  (Default|Despawn (Variables|Default|GetGlassesSpawner) Glass))

(fn RespawnCharacter
  (params (Character :type BP%20Ice%20Cube%20Character%20Object%20Reference))
  (bind _glassesspawner (Variables|Default|GetGlassesSpawner))
  (bind _spawnedglasses (Variables|/Game/ScoreSpace/Glasses/BP_GlassesSpawner.BP_GlassesSpawner_C|GetSpawnedGlasses _glassesspawner))
  (Default|OnRespawn Character (+ (Transformation|GetWorldLocation (Variables|/Game/ScoreSpace/Glasses/BP_Glass.BP_Glass_C|GetDefaultSceneRoot (Utilities|Array|Get(acopy) _spawnedglasses (/ (Utilities|Array|Length _spawnedglasses) 2)))) (Math|Vector|MakeVector 0.0 0.0 (LocalVariables|GetRespawnOffsetZ)))))